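; Player controller that lets the player collect pickups by clicking or touching them, adding their items to an inventory array.
; Left click and touch share a Visibility line trace deprojected from the mouse position, drawn as a one-frame debug line.
; A hit BP_PickupMaster actor tagged "Pickup" passes its Item to AddItem, which appends it to PlayerSlot, and is then destroyed.
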(event `Key|LeftMouseButton`
  (params (Key :type "Key Structure"))
  (bind (_worldlocation _worlddirection) (`self.DeprojectMousePositionToWorld`))
  ;[1 1 1] pickup
  (:`Pressed`
    (bind (_outhit _returnvalue) (`KismetSystemLibrary.LineTraceSingle` :`Start` _worldlocation :`End` (* (+ (`SceneComponent.GetForwardVector` (`PlayerCameraManager.TransformComponent` (`GameplayStatics.GetPlayerCameraManager` 0))) 300000) _worlddirection) :`TraceChannel` "TraceTypeQuery1" :`DrawDebugType` "ForOneFrame" :!label _label))
    (if _returnvalue
      (bind (_bblockinghit _binitialoverlap _time _distance _location _impactpoint _normal _impactnormal _physmat _hitactor) (`GameplayStatics.BreakHitResult` _outhit))
      (bind _asbp_pickup_master (cast `/Game/JY/Blueprints/BP_BeforeRoom/BeforeRoomBlueprint/BP_PickupMaster` _hitactor))
      (if (`self.ActorHasTag` _hitactor "Pickup")
        (`self.AddItem` (`/Game/JY/Blueprints/BP_BeforeRoom/BeforeRoomBlueprint/BP_PickupMaster.item` _asbp_pickup_master))
        (`self.K2_DestroyActor` _asbp_pickup_master)))))

(event `InputTouch`
  (params (Location :type "Vector Structure") (FingerIndex :type "ETouchIndex Enum"))
  ;[1 1 1] pickup
  (:`Pressed`
    (goto _label)))

(fn `AddItem`
  (params (pickupItem :type "/Game/JY/Blueprints/S_Slot Structure"))
  (`KismetArrayLibrary.Array_Add` (`self.PlayerSlot`) pickupItem))

(fn `UserConstructionScript`)