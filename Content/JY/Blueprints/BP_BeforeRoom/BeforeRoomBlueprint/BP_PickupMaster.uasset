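; BP_PickupMaster is a pickup item actor configured through a data table row handle.
; The Construction Script looks up that row and assigns its static mesh to the mesh component.
; Clicking or touching the mesh looks up the row again and branches on the item number, so far only printing the item name for the first two numbers.
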(event `self.StaticMeshComponent.OnInputTouchBegin`
  (params (FingerIndex :type "ETouchIndex Enum" :default "Touch1") (TouchedComponent :type "PrimitiveComponent Object Reference"))
  (bind (_datatable _rowname) (break `DataTableRowHandle` (`.item_8_16478CC34F520FEDD06C318FD6F06E5C` (break `/Game/JY/Blueprints/S_Slot` (`self.item`)))))
  ;[1 1 1] 번호에 맞는 item 눌렀을때
  (bind _returnvalue (`|GetDataTableRow` _datatable _rowname :!label _label)
    (:`then`
      (bind (_itemname _itemtexture _itemstaticmesh _itemnum) (break `/Game/JY/Blueprints/S_Inventory` _returnvalue))
      (if (== _itemnum 1)
        (`KismetSystemLibrary.PrintString` _itemname)
        (elif (== _itemnum 2)
          (`KismetSystemLibrary.PrintString` _itemname))))))

(event `self.StaticMeshComponent.OnClicked`
  (params (TouchedComponent :type "PrimitiveComponent Object Reference") (ButtonPressed :type "Key Structure"))
  ;[1 1 1] 번호에 맞는 item 눌렀을때
  (goto _label))

(fn `UserConstructionScript`
  (bind (_datatable _rowname) (break `DataTableRowHandle` (`.item_8_16478CC34F520FEDD06C318FD6F06E5C` (break `/Game/JY/Blueprints/S_Slot` (`self.item`)))))
  (bind _returnvalue (`|GetDataTableRow` _datatable _rowname)
    (:`then`
      (`StaticMeshComponent.SetStaticMesh` (`self.StaticMeshComponent`) (`.itemStaticmesh_14_EA5B032D451C283EC75D68AF300AC547` (break `/Game/JY/Blueprints/S_Inventory` _returnvalue))))))