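; Opening-room interactive prop that responds to mouse clicks and touches on two mesh components.
; Selecting the main StaticMesh prints a debug string and switches the player's view target to the owner of the CineCamera component.
; Selecting CloseDrawer calls FirstOpen, which is not defined in this graph, then calls SetStaticMesh on the drawer with no mesh specified.
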(event `self.StaticMesh.OnInputTouchBegin`
  (params (FingerIndex :type "ETouchIndex Enum" :default "Touch1") (TouchedComponent :type "PrimitiveComponent Object Reference"))
  (`KismetSystemLibrary.PrintString` "Hello_0" :!label _label)
  (`PlayerController.SetViewTargetWithBlend` (`GameplayStatics.GetPlayerController` 0) (`ActorComponent.GetOwner` (`self.CineCamera`)) 0.0 "VTBlend_Linear" 0.0 false))

(event `self.StaticMesh.OnClicked`
  (params (TouchedComponent :type "PrimitiveComponent Object Reference") (ButtonPressed :type "Key Structure"))
  (goto _label))

(event `self.closeDrawer.OnInputTouchBegin`
  (params (FingerIndex :type "ETouchIndex Enum" :default "Touch1") (TouchedComponent :type "PrimitiveComponent Object Reference"))
  (`self.FirstOpen` :!label _label_2)
  (`StaticMeshComponent.SetStaticMesh` (`self.closeDrawer`) null))

(event `self.closeDrawer.OnClicked`
  (params (TouchedComponent :type "PrimitiveComponent Object Reference") (ButtonPressed :type "Key Structure"))
  (goto _label_2))

(fn `UserConstructionScript`)